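; BP_PointItem is a collectible that awards points to the overlapping actor, then plays a sound and destroys itself.
; The construction script reads the point value and mesh material from a DT_PointItem row chosen by name.
; Two timelines animate the mesh's yaw spin and vertical motion.
; Pickup fires on the box's end overlap, not begin, sending the item's name and points through CharacterHitActionMessage.
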(event OnComponentEndOverlap(Box)
  (params (OverlappedComponent :type Primitive%20Component%20Object%20Reference) (OtherActor :type Actor%20Object%20Reference) (OtherComp :type Primitive%20Component%20Object%20Reference) (OtherBodyIndex :type Integer))
  (Class|BPIMycharacter|CharacterHitAction(Message) OtherActor (Utilities|GetDisplayName self) (Variables|Default|GetPoint))
  (Audio|PlaySoundatLocation 0 (Transformation|GetActorLocation) "0, 0, 0" 1.0 1.0 0.0 0 0 0 0)
  (Actor|DestroyActor))

(event EventBeginPlay
  (Utilities|FlowControl|Sequence
    (:then_0
      (bind _rotate (Timeline|Rotate Play)
        (:Update
          (if (< (Variables|Default|GetActet%20Rotation) 3.6e+02)
            (Variables|Default|SetActet%20Rotation _rotate)
            (else
              (Variables|Default|SetActet%20Rotation 0.0)))
          (Transformation|SetRelativeRotation (Variables|Default|GetSTM_PointItem) (Math|Rotator|MakeRotator 0.0 0.0 (Variables|Default|GetActet%20Rotation)) false false))))
    (:then_1
      (bind _movingvalue (Timeline|Moving Play)
        (:Update
          (Transformation|SetRelativeLocation (Variables|Default|GetSTM_PointItem) (Math|Vector|MakeVector 0.0 0.0 _movingvalue) false false))))))

(fn ConstructionScript
  (bind _returnvalue (Utilities|GetDataTableRow "/Game/Project/Blueprints/DT_PointItem.DT_PointItem" (Variables|Default|GetPointItemDataName))
    (:then
      (Variables|Default|SetPoint (.Point (Utilities|Struct|BreakST_PointItem _returnvalue)))
      (Rendering|Material|SetMaterial (Variables|Default|GetSTM_PointItem) 0 (.Material (Utilities|Struct|BreakST_PointItem _returnvalue))))))