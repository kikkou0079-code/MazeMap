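; BP_TargetBox is a trigger actor that sets three referenced moving objects in motion when an actor leaves its box.
; On end overlap it reports its name with zero points to the leaving actor, then messages each moving object, all through interface-style calls.
; A DestroyTestBox event destroys the box itself, while a similar destroy message to DestroyTargetActor is left unconnected and never runs.
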(event OnComponentEndOverlap(Box)
  (params (OverlappedComponent :type Primitive%20Component%20Object%20Reference) (OtherActor :type Actor%20Object%20Reference) (OtherComp :type Primitive%20Component%20Object%20Reference) (OtherBodyIndex :type Integer))
  (Class|BPIMycharacter|CharacterHitAction(Message) OtherActor (Utilities|GetDisplayName self))
  (Class|BPIMovementObject|MovingtObject(Message) (Variables|Default|GetMoving%20Object_1))
  (Class|BPIMovementObject|MovingtObject(Message) (Variables|Default|GetMoving%20Object%20_2))
  (Class|BPIMovementObject|MovingtObject(Message) (Variables|Default|GetMoving%20Object%20_3)))

(event EventDestroyTestBox
  (Actor|DestroyActor))

(fn ConstructionScript)